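; Inventory component that holds a fixed number of item slots, sized on BeginPlay, and toggles an inventory widget.
; Adding an item tops up a matching partial stack, recursing with any overflow, or otherwise fills the first empty slot.
; Adding to an existing stack always reports success, even if the overflow finds no space.
; The toggle attaches the widget to the player character's HUD canvas and switches input mode and mouse cursor.
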(event `self.ReceiveBeginPlay`
  (`KismetArrayLibrary.Array_Resize` (`self.Inventory`) (`self.NumberOfSlots`)))

(fn `Fucn_AddToInventory`
  (params (ItemsToAdd :type "/Game/Struct/Struct_Slot Structure"))
  (returns (Success :type Boolean))
  (if (`.IsStackable_13_6157352F4123C2616FB2F7B1481A5D6E` (break `/Game/Struct/Struct_Item` (`.ItemStructure_3_40CC9EAE492771523FEEBA99829E43F1` (break `/Game/Struct/Struct_Slot` ItemsToAdd))))
    (bind _slotindex (`self.HasPartialStack` ItemsToAdd)
      (:`True`
        (bind _success (`self.Func_AddToStack` (`local.ItemsToAdd`) _slotindex))
        (set `self.bIsSuccess` _success))
      (:`False`
        (bind _success_2 (`self.Func_CreateStack` ItemsToAdd :!label _label))
        (set `self.bIsSuccess` _success_2)))
    (else
      (goto _label)))
  (return (`self.bIsSuccess`)))

(fn `Func_AddToStack`
  (params (Slot :type "/Game/Struct/Struct_Slot Structure") (Index :type Integer))
  (returns (Success :type Boolean))
  (locals (CurrentInteger :type Integer))
  (bind (_slot_itemstructure _slot_quantity) (break `/Game/Struct/Struct_Slot` (`local.Slot`)))
  (bind _slot_itemstructure_2 (break `/Game/Struct/Struct_Slot` (`local.Slot`)))
  (bind _inventory (`self.Inventory`))
  (bind _index (`local.Index`))
  (bind (_slot_itemstructure_3 _slot_quantity_2) (break `/Game/Struct/Struct_Slot` (`local.Slot`)))
  (bind (_itemname _itemdescription _canbeadded _itemicon _isstackable _ispickupbeneficial _itemclass _maxstacksize) (break `/Game/Struct/Struct_Item` _slot_itemstructure_2))
  (bind (_output_itemstructure _output_quantity) (break `/Game/Struct/Struct_Slot` (`|GetArrayItem` _inventory _index)))
  (bind _output (`|GetArrayItem` (`self.Inventory`) Index))
  (bind _output_get (set `local.CurrentInteger` (`.Quantity_5_3E25FE604C38C89B6A05CC877C79A408` (break `/Game/Struct/Struct_Slot` _output))))
  (if (> (+ _output_get (`.Quantity_5_3E25FE604C38C89B6A05CC877C79A408` (break `/Game/Struct/Struct_Slot` Slot))) (`.MaxStackSize_22_A25FE13844194E4512D315B15B729889` (break `/Game/Struct/Struct_Item` (break `/Game/Struct/Struct_Slot` _output))))
    (`KismetArrayLibrary.Array_Set` (`self.Inventory`) (`local.Index`) (make `/Game/Struct/Struct_Slot` _slot_itemstructure_2 _maxstacksize))
    (`self.Fucn_AddToInventory` (make `/Game/Struct/Struct_Slot` (struct) (- _slot_quantity (- _maxstacksize (`local.CurrentInteger`)))))
    (else
      (`KismetArrayLibrary.Array_Set` _inventory _index (make `/Game/Struct/Struct_Slot` _output_itemstructure (+ _output_quantity _slot_quantity_2)))))
  (return true))

(fn `Func_CreateStack`
  (params (Slot :type "/Game/Struct/Struct_Slot Structure"))
  (returns (Success :type Boolean))
  (locals (EmptyIndex :type Integer))
  (for (_array_element _array_index) (`self.Inventory`)
    (if (<= (`.Quantity_5_3E25FE604C38C89B6A05CC877C79A408` (break `/Game/Struct/Struct_Slot` _array_element)) 0)
      (set `self.bHasSpace` true)
      (set `local.EmptyIndex` _array_index)
      (break)))
  (if (`self.bHasSpace`)
    (`KismetArrayLibrary.Array_Set` (`self.Inventory`) (`local.EmptyIndex`) (`local.Slot`))
    (return (`self.bHasSpace`))
    (else
      (return false))))

(fn `Func_ToggleInventory`
  (bind _returnvalue (`GameplayStatics.GetPlayerController` 0))
  (bind _returnvalue_2 (`GameplayStatics.GetPlayerController` 0))
  (bind _wbp_inventory (`self.WBP_Inventory`)
    (:`then`
      (`Widget.RemoveFromParent` _wbp_inventory)
      (set `self.WBP_Inventory` null)
      (`WidgetBlueprintLibrary.SetInputMode_GameOnly` _returnvalue)
      (set `PlayerController.bShowMouseCursor` false _returnvalue))
    (:`else`
      (bind _returnvalue_3 (`|CreateWidget` "/Game/UI/WBP_Inventory.WBP_Inventory_C" null self (`self.InventoryName`)))
      (bind _output_get (set `self.WBP_Inventory` _returnvalue_3))
      (bind _asbp_base_character (cast `/Game/BP_BaseCharacter` (`GameplayStatics.GetPlayerCharacter` 0)))
      (bind _wbp_hud (`/Game/BP_BaseCharacter.WBP_HUD` _asbp_base_character)
        (:`then`
          (bind _returnvalue_4 (`CanvasPanel.AddChildToCanvas` (`/Game/UI/WBP_HUD.Canvas` _wbp_hud) _output_get))
          (`CanvasPanelSlot.SetAutoSize` _returnvalue_4 true)
          (`CanvasPanelSlot.SetAlignment` _returnvalue_4 (0.5 0.5))
          (`CanvasPanelSlot.SetAnchors` _returnvalue_4 (make `Anchors` (0.6 0.1) (1.0 1.0)))
          (`WidgetBlueprintLibrary.SetInputMode_UIOnlyEx` _returnvalue_2 _output_get)
          (set `PlayerController.bShowMouseCursor` true _returnvalue_2))
        (:`else`)))))