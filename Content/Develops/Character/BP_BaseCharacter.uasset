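; Player character with Enhanced Input movement, dash, trace-driven montage parkour, inventory, HUD widgets and timed health regeneration.
; Aiming holds a sphere projectile launched on release, while shooting sustains a timer-steered beam, both targeted by a camera trace.
; A per-tick sphere trace finds BPI_Inspect actors for interaction.
; A looping timer polls Ultra Dynamic Sky to apply an ice material and Niagara effect at night, alongside debug keys.
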(event `Look`
  (bind _mesh (`self.Mesh`))
  (bind _ns_ice (`self.NS_Ice`))
  ;[0.15 0.02562 0.004951 0.5] TEST
  (`KismetSystemLibrary.K2_SetTimerDelegate` (delegate `Look`) 0.5 true true)
  (if (`/Game/UltraDynamicSky/Blueprints/Functions/UltraDynamicSky_Functions.Is It Daytime? · 𝖴𝖣𝖲`)
    (`PrimitiveComponent.SetMaterial` _mesh 0 "/Game/TestChar/Ch14_Body.Ch14_Body")
    (`SceneComponent.SetVisibility` _ns_ice false false)
    (else
      (`PrimitiveComponent.SetMaterial` _mesh 0 "/Game/Art/MateriaAndVFX/MI/M_Ice_Inst.M_Ice_Inst")
      (`SceneComponent.SetVisibility` _ns_ice true false))))

(event `self.ReceiveBeginPlay`
  (`|ExecutionSequence`
    (:`then_0`
      (bind _asplayer_controller (cast `PlayerController` (`self.GetController`)))
      (`EnhancedInputSubsystemInterface.AddMappingContext` (pcsubsystem `EnhancedInputLocalPlayerSubsystem` _asplayer_controller) "/Game/Develops/Input/IMC_Keeper.IMC_Keeper" 0 (struct)))
    (:`then_1`
      (bind _returnvalue (`|CreateWidget` "/Game/UI/MainScreenWidgets/WBP_MainScreen.WBP_MainScreen_C"))
      (bind _output_get (set `self.WBP_MainScreen` _returnvalue))
      (`UserWidget.AddToViewport` _output_get 0)
      (`self.CreateHealth`)
      (`self.Look`))
    (:`then_2`
      (bind _returnvalue_2 (`|CreateWidget` "/Game/UI/MainScreenWidgets/WBP_HUD.WBP_HUD_C"))
      (bind _output_get_2 (set `self.WBP_HUD` _returnvalue_2))
      (`UserWidget.AddToViewport` _output_get_2 0))))

(event `Key|Tab`
  (params (Key :type "Key Structure"))
  ;[0.15 0.02562 0.004951 0.5] TEST
  (:`Pressed`
    (`/Game/UltraDynamicSky/Blueprints/Functions/UltraDynamicSky_Functions.Transition Time of Day · 𝖴𝖣𝖲` 1000.0 5.0 "EaseInOut" 2.0 true)
    (`KismetSystemLibrary.PrintString` "New day")))

(event `EnhancedInput|/Game/Develops/Input/IA/IA_Parkour`
  (params (ActionValue :type Boolean) (ElapsedSeconds :type "Float (double-precision)") (TriggeredSeconds :type "Float (double-precision)") (InputAction :type "InputAction Object Reference" :default "/Game/Develops/Input/IA/IA_Parkour.IA_Parkour"))
  ;[0.15 0.02562 0.004951 0.5] TEST
  (:`Started`
    (`self.Parkour`)))

(event `EnhancedInput|/Game/Develops/Input/IA/IA_Move`
  (params (ActionValue :type "Vector2D Structure") (ElapsedSeconds :type "Float (double-precision)") (TriggeredSeconds :type "Float (double-precision)") (InputAction :type "InputAction Object Reference" :default "/Game/Develops/Input/IA/IA_Move.IA_Move"))
  (bind (_returnvalue_roll _returnvalue_pitch _returnvalue_yaw) (`KismetMathLibrary.BreakRotator` (`self.GetControlRotation`)))
  (bind (_returnvalue_roll_2 _returnvalue_pitch_2 _returnvalue_yaw_2) (`KismetMathLibrary.BreakRotator` (`self.GetControlRotation`)))
  (:`Triggered`
    (`self.AddMovementInput` (`KismetMathLibrary.GetRightVector` (`KismetMathLibrary.MakeRotator` _returnvalue_roll_2 0.0 _returnvalue_yaw_2)) ActionValue_X)
    (`self.AddMovementInput` (`KismetMathLibrary.GetForwardVector` (`KismetMathLibrary.MakeRotator` 0.0 0.0 _returnvalue_yaw)) ActionValue_Y)))

(event `EnhancedInput|/Game/Develops/Input/IA/IA_Look`
  (params (ActionValue :type "Vector2D Structure") (ElapsedSeconds :type "Float (double-precision)") (TriggeredSeconds :type "Float (double-precision)") (InputAction :type "InputAction Object Reference" :default "/Game/Develops/Input/IA/IA_Look.IA_Look"))
  (:`Triggered`
    (`self.AddControllerYawInput` ActionValue_X)
    (`self.AddControllerPitchInput` ActionValue_Y)))

(event `EnhancedInput|/Game/Develops/Input/IA/IA_Aiming`
  (params (ActionValue :type Boolean) (ElapsedSeconds :type "Float (double-precision)") (TriggeredSeconds :type "Float (double-precision)") (InputAction :type "InputAction Object Reference" :default "/Game/Develops/Input/IA/IA_Aiming.IA_Aiming"))
  (:`Triggered`
    (if (not (`self.bIsShoot`))
      (set `self.bIsAiming` true)
      (set `self.bUseControllerRotationYaw` true)
      (`self.Func_LineTrace`)
      (`/Engine/EditorBlueprintResources/StandardMacros.DoOnce` false :!label _label
        (:`Completed`
          (bind _returnvalue (`|SpawnActorFromClass` "/Game/Develops/FVXBP/BP_Sphere.BP_Sphere_C" (`KismetMathLibrary.MakeTransform` (`SceneComponent.K2_GetComponentLocation` (`self.Scene`))) "Undefined" "MultiplyWithRoot" null null))
          (bind _output_get (set `self.BP_Sphere` _returnvalue))
          (`self.K2_AttachToComponent` _output_get (`self.Scene`) "None" "SnapToTarget" "SnapToTarget" "KeepRelative" true)
          (set `self.bIsSphere` true)))))
  (:`Canceled`
    (set `self.bIsAiming` false :!label _label_2)
    (set `self.bUseControllerRotationYaw` false)
    (if (`self.bIsSphere`)
      (`self.Func_ShootSphere`)
      (set `self.bIsSphere` false)
      (`SceneComponent.K2_DetachFromComponent` (`Actor.RootComponent` (`self.BP_Sphere`)) "KeepWorld" "KeepWorld" "KeepRelative" true)
      (goto _label :!via `Reset`)))
  (:`Completed`
    (goto _label_2)))

(event `EnhancedInput|/Game/Develops/Input/IA/IA_Shoot`
  (params (ActionValue :type Boolean) (ElapsedSeconds :type "Float (double-precision)") (TriggeredSeconds :type "Float (double-precision)") (InputAction :type "InputAction Object Reference" :default "/Game/Develops/Input/IA/IA_Shoot.IA_Shoot"))
  (:`Triggered`
    (if (not (`self.bIsAiming`))
      (set `self.bIsShoot` true)
      (`self.Func_LineTrace`)
      (set `self.bUseControllerRotationYaw` true)
      (`/Engine/EditorBlueprintResources/StandardMacros.DoOnce` false :!label _label_3
        (:`Completed`
          (bind _returnvalue (`|SpawnActorFromClass` "/Game/Develops/FVXBP/BP_Beam.BP_Beam_C" (`KismetMathLibrary.MakeTransform` (`SceneComponent.K2_GetComponentLocation` (`self.Scene`))) "Undefined" "MultiplyWithRoot" null null))
          (bind _output_get (set `self.BP_Beam` _returnvalue))
          (`self.K2_AttachToComponent` _output_get (`self.Scene`) "None" "SnapToTarget" "SnapToTarget" "KeepRelative" true)
          (bind _returnvalue_2 (`KismetSystemLibrary.K2_SetTimerDelegate` (delegate `Beam`) 0.02 true))
          (set `self.BeamTimer` _returnvalue_2)))))
  (:`Canceled`
    (set `self.bIsShoot` false :!label _label_4)
    (bind _bp_beam (`self.BP_Beam`)
      (:`then`
        (`self.K2_DestroyActor` _bp_beam)
        (set `self.bUseControllerRotationYaw` false)
        (`KismetSystemLibrary.K2_ClearAndInvalidateTimerHandle` (`self.BeamTimer`))
        (goto _label_3 :!via `Reset`))
      (:`else`)))
  (:`Completed`
    (goto _label_4)))

(event `Beam`
  (if (`self.bIsHit`)
    (bind _bp_beam (`self.BP_Beam`)
      (:`then`
        (`SceneComponent.K2_SetWorldRotation` (`/Game/Develops/FVXBP/BP_Beam.NS_Beam` _bp_beam) (`KismetMathLibrary.FindLookAtRotation` (`SceneComponent.K2_GetComponentLocation` (`self.Scene`)) (`self.Impact Point`)) false false))
      (:`else`))
    (else
      (bind _bp_beam_2 (`self.BP_Beam`)
        (:`then`
          (`SceneComponent.K2_SetWorldRotation` (`/Game/Develops/FVXBP/BP_Beam.NS_Beam` _bp_beam_2) (`KismetMathLibrary.FindLookAtRotation` (`SceneComponent.K2_GetComponentLocation` (`self.Scene`)) (`self.Trace End`)) false false))
        (:`else`)))))

(event `EnhancedInput|/Game/Develops/Input/IA/IA_Dash`
  (params (ActionValue :type Boolean) (ElapsedSeconds :type "Float (double-precision)") (TriggeredSeconds :type "Float (double-precision)") (InputAction :type "InputAction Object Reference" :default "/Game/Develops/Input/IA/IA_Dash.IA_Dash"))
  (:`Started`
    (`self.K2_SetActorLocation` (+ (`self.K2_GetActorLocation`) (* (`self.GetActorForwardVector`) 1500.0)) true)))

(event `Key|One`
  (params (Key :type "Key Structure"))
  (:`Pressed`
    (bind _health (`/Game/Develops/Core/ActorComponents/AC_Health.Func_Hit` (`self.AC_Health`)))
    (`ProgressBar.SetPercent` (`/Game/UI/MainScreenWidgets/WBP_MainScreen.PG_HealthBar` (`self.WBP_MainScreen`)) _health)))

(event `CreateHealth`
  (bind _ac_health (`self.AC_Health`))
  (bind _returnvalue (`KismetMathLibrary.FClamp` (+ (`/Game/Develops/Core/ActorComponents/AC_Health.Health` _ac_health) 0.3)))
  (bind _returnvalue_2 (`KismetSystemLibrary.K2_SetTimerDelegate` (delegate `CreateHealth`) 3.0 true))
  (set `self.HealthTimer` _returnvalue_2)
  (if (<= (`/Game/Develops/Core/ActorComponents/AC_Health.Health` (`self.AC_Health`)) 0.9)
    (`KismetSystemLibrary.PrintString` (`KismetStringLibrary.Conv_DoubleToString` _returnvalue))
    (bind _output_get (set `/Game/Develops/Core/ActorComponents/AC_Health.Health` _returnvalue _ac_health))
    (`ProgressBar.SetPercent` (`/Game/UI/MainScreenWidgets/WBP_MainScreen.PG_HealthBar` (`self.WBP_MainScreen`)) _output_get)))

(event `self.ReceiveTick`
  (params (DeltaSeconds :type "Float (single-precision)"))
  (`self.Func_StartTrace`))

(event `EnhancedInput|/Game/Develops/Input/IA/IA_Interact`
  (params (ActionValue :type Boolean) (ElapsedSeconds :type "Float (double-precision)") (TriggeredSeconds :type "Float (double-precision)") (InputAction :type "InputAction Object Reference" :default "/Game/Develops/Input/IA/IA_Interact.IA_Interact"))
  (:`Triggered`
    (set `self.bIsItem` true)
    (bind _traceitem (`self.TraceItem`)
      (:`then`
        (message `/Game/Develops/Interfaces/BPI_Inspect.Interact Items` _traceitem self))
      (:`else`)))
  (:`Canceled`
    (set `self.bIsItem` false :!label _label_5))
  (:`Completed`
    (goto _label_5)))

(event `EnhancedInput|/Game/Develops/Input/IA/IA_Inventory`
  (params (ActionValue :type Boolean) (ElapsedSeconds :type "Float (double-precision)") (TriggeredSeconds :type "Float (double-precision)") (InputAction :type "InputAction Object Reference" :default "/Game/Develops/Input/IA/IA_Inventory.IA_Inventory"))
  (:`Triggered`
    (`/Game/Develops/Core/ActorComponents/AC_Inventory.Func_ToggleInventory` (`self.AC_Inventory`))))

(event `EnhancedInput|/Game/Develops/Input/IA/IA_Jump`
  (params (ActionValue :type Boolean) (ElapsedSeconds :type "Float (double-precision)") (TriggeredSeconds :type "Float (double-precision)") (InputAction :type "InputAction Object Reference" :default "/Game/Develops/Input/IA/IA_Jump.IA_Jump"))
  (:`Started`
    (`self.Jump`))
  (:`Canceled`
    (`self.StopJumping` :!label _label_6))
  (:`Completed`
    (goto _label_6)))

(fn `Func_LineTrace`
  (bind _returnvalue (`GameplayStatics.GetPlayerCameraManager` 0))
  (bind _returnvalue_2 (`self.K2_GetActorLocation` _returnvalue))
  (bind _outactors (`GameplayStatics.GetAllActorsOfClass` "/Game/Develops/FVXBP/BP_Sphere.BP_Sphere_C"))
  (bind _output_get (set `self.IgnorActor` _outactors))
  (bind _outhit (`KismetSystemLibrary.LineTraceSingle` _returnvalue_2 (+ _returnvalue_2 (* (`self.GetActorForwardVector` _returnvalue) 50000.0)) "TraceTypeQuery1" false _output_get "None" true (struct :`R` 1.0 :`G` 0.085438 :`B` 0.816395 :`A` 1.0)))
  (bind (_bblockinghit _binitialoverlap _time _distance _location _impactpoint _normal _impactnormal _physmat _hitactor _hitcomponent _hitbonename _bonename _hititem _elementindex _faceindex _tracestart _traceend) (`GameplayStatics.BreakHitResult` _outhit))
  (bind _output_get_2 (set `self.bIsHit` _bblockinghit))
  (if _output_get_2
    (bind _output_get_3 (set `self.Impact Point` _location))
    (`KismetSystemLibrary.LineTraceSingle` (`SceneComponent.K2_GetComponentLocation` (`self.Scene`)) _output_get_3 "TraceTypeQuery1" false (`self.IgnorActor`) "ForDuration" true (struct :`R` 0.006112 :`G` 0.339101 :`B` 1.0 :`A` 1.0))
    (else
      (bind _output_get_4 (set `self.Trace End` _traceend))
      (`KismetSystemLibrary.LineTraceSingle` (`SceneComponent.K2_GetComponentLocation` (`self.Scene`)) _output_get_4 "TraceTypeQuery1" false (`self.IgnorActor`) "ForDuration" true (struct :`R` 0.765964 :`G` 1.0 :`B` 0.073219 :`A` 1.0)))))

(fn `Func_ShootSphere`
  (bind _bp_sphere (`self.BP_Sphere`))
  (bind _bp_sphere_2 (`self.BP_Sphere`)
    (:`then`
      (set `self.StartLocation` (`SceneComponent.K2_GetComponentLocation` (`Actor.RootComponent` _bp_sphere_2)))
      (if (`self.bIsHit`)
        (bind _projectilemovement (`/Game/Develops/FVXBP/BP_Sphere.ProjectileMovement` _bp_sphere_2))
        (set `MovementComponent.Velocity` (* (`KismetMathLibrary.Normal` (- (`self.Impact Point`) (`self.StartLocation`))) 1800.0) _projectilemovement)
        (`self.SetLifeSpan` _bp_sphere 30.0)
        (else
          (set `MovementComponent.Velocity` (* (`KismetMathLibrary.Normal` (- (`self.Trace End`) (`self.StartLocation`))) 1800.0) _projectilemovement)
          (`self.SetLifeSpan` _bp_sphere 30.0))))
    (:`else`)))

(fn `Func_StartTrace`
  (bind _capsulecomponent (`self.CapsuleComponent`))
  (bind _relativelocation (`SceneComponent.RelativeLocation` _capsulecomponent))
  (bind _outhit (`KismetSystemLibrary.SphereTraceSingle` _relativelocation (+ _relativelocation (* (`SceneComponent.GetForwardVector` _capsulecomponent) 200.0)) 50.0 "TraceTypeQuery1"))
  (bind (_bblockinghit _binitialoverlap _time _distance _location _impactpoint _normal _impactnormal _physmat _hitactor) (`GameplayStatics.BreakHitResult` _outhit))
  (if (`KismetSystemLibrary.DoesImplementInterface` _hitactor "/Game/Develops/Interfaces/BPI_Inspect.BPI_Inspect_C")
    (if (!= _hitactor (`self.TraceItem`))
      (bind _output_get (set `self.TraceItem` _hitactor)))
    (message `/Game/Develops/Interfaces/BPI_Inspect.Can Recieve Traces` _output_get true)
    (else
      (bind _traceitem (`self.TraceItem`)
        (:`then`
          (message `/Game/Develops/Interfaces/BPI_Inspect.Can Recieve Traces` _traceitem false)
          (set `self.TraceItem` null))
        (:`else`)))))

(fn `UserConstructionScript`)