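; Base interactable item that players pick up into their inventory or consume on the spot.
; A sphere overlap with the Player shows a WBP_Interact widget, and trace events toggle its highlight border.
; Interaction adds the item struct to AC_Inventory or calls the pick-up-benefit function, destroying the actor on success.
; Benefit and use functions are stubs returning false; BP_Studio inspection logic exists but is disconnected.
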(event `self.ReceiveBeginPlay`
  (setmembers `/Game/Develops/Struct/Struct_Item` :`StructRef` (`self.ItemStructure`) :`Mesh` (`StaticMeshComponent.StaticMesh` (`self.StaticMesh`))))

(event `self.Sphere.OnComponentBeginOverlap`
  (params (OverlappedComponent :type "PrimitiveComponent Object Reference") (OtherActor :type "Actor Object Reference") (OtherComp :type "PrimitiveComponent Object Reference") (OtherBodyIndex :type Integer) (bFromSweep :type Boolean) (SweepResult :type "HitResult Structure (by ref)"))
  (bind _widget (`self.Widget`))
  (if (`self.ActorHasTag` OtherActor "Player")
    (bind _returnvalue (`|CreateWidget` "/Game/UI/InteractiveWidgets/InventoryWidgets/WBP_Interact.WBP_Interact_C"))
    (bind _output_get (set `self.WBP_Interact` _returnvalue))
    (`WidgetComponent.SetWidget` _widget _output_get)
    (`SceneComponent.SetVisibility` _widget true false)))

(event `self.Sphere.OnComponentEndOverlap`
  (params (OverlappedComponent :type "PrimitiveComponent Object Reference") (OtherActor :type "Actor Object Reference") (OtherComp :type "PrimitiveComponent Object Reference") (OtherBodyIndex :type Integer))
  (if (`self.ActorHasTag` OtherActor "Player")
    (bind _wbp_interact (`self.WBP_Interact`)
      (:`then`
        (`Widget.RemoveFromParent` _wbp_interact)
        (set `self.WBP_Interact` null)
        (`SceneComponent.SetVisibility` (`self.Widget`) false false))
      (:`else`))))

(event `/Game/Develops/Interfaces/BPI_Inspect.Can Recieve Traces`
  (params (`Can Interact` :type Boolean))
  (if `Can Interact`
    (bind _wbp_interact (`self.WBP_Interact`)
      (:`then`
        (`Widget.SetRenderOpacity` (`/Game/UI/InteractiveWidgets/InventoryWidgets/WBP_Interact.Interaction_Border` _wbp_interact) 1.0))
      (:`else`))
    (else
      (bind _wbp_interact_2 (`self.WBP_Interact`)
        (:`then`
          (`Widget.SetRenderOpacity` (`/Game/UI/InteractiveWidgets/InventoryWidgets/WBP_Interact.Interaction_Border` _wbp_interact_2) 0.0))
        (:`else`)))))

(event `/Game/Develops/Interfaces/BPI_Inspect.Interact Items`
  (params (Player :type "/Game/Develops/Character/BP_BaseCharacter Object Reference"))
  (bind (_itemstructure_itemname _itemstructure_itemdescription _itemstructure_canbeadded _itemstructure_itemicon _itemstructure_isstackable _itemstructure_ispickupbeneficial) (break `/Game/Develops/Struct/Struct_Item` (`self.ItemStructure`)))
  (if _itemstructure_canbeadded
    (bind _success (`/Game/Develops/Core/ActorComponents/AC_Inventory.Fucn_AddToInventory` (`self.GetComponentByClass` Player "/Game/Develops/Core/ActorComponents/AC_Inventory.AC_Inventory_C") (make `/Game/Develops/Struct/Struct_Slot` (`self.ItemStructure`) 1)))
    (if _success
      (`self.K2_DestroyActor` :!label _label))
    (elif _itemstructure_ispickupbeneficial
      (bind _success_2 (`self.Func_PickUpBeneficial`))
      (if _success_2
        (goto _label)))))

(fn `Func_PickUpBeneficial`
  (returns (Success :type Boolean))
  (return false))

(fn `Func_UseItems`
  (returns (Success :type Boolean))
  (return false))

(fn `UserConstructionScript`)