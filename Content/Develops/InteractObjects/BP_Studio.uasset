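; Temporary studio actor for inspecting an item in 3D, opened from the inventory UI or elsewhere.
; Inspect sets the mesh, shows WBP_Inspection with name and description, and moves input from the player to itself.
; Shoot-drag or Move input rotates the item, while the mouse wheel zooms through the SceneCaptureComponent2D's clamped FOV.
; Interact restores player input, removes the widget, destroys the actor and refocuses the inventory when opened from it.
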(event `/Game/Develops/Interfaces/BPI_Inspect.Inspect`
  (params (Player :type "/Game/Develops/Character/BP_BaseCharacter Object Reference") (ItemToFocus :type "StaticMesh Object Reference") (ItemName :type Text) (ItemDescription :type Text) (`From UI` :type Boolean) (UI :type "/Game/UI/InteractiveWidgets/InventoryWidgets/WBP_Inventory Object Reference"))
  (bind _returnvalue (`GameplayStatics.GetPlayerController` 0))
  (set `self.BP_Player` Player)
  (`StaticMeshComponent.SetStaticMesh` (`self.Item`) ItemToFocus)
  (set `self.bIsFromUI` `From UI`)
  (set `self.WBP_Inventory` UI)
  (`GameplayStatics.PlaySound2D` "/Engine/VREditor/Sounds/UI/Click_on_Button_Cue.Click_on_Button_Cue" 1.0 1.0 0.0 null null)
  (bind _returnvalue_2 (`|CreateWidget` "/Game/UI/InteractiveWidgets/InventoryWidgets/WBP_Inspection.WBP_Inspection_C" null ItemName ItemDescription))
  (bind _output_get (set `self.WBP_Inspection` _returnvalue_2))
  (`UserWidget.AddToViewport` _output_get 0)
  (`self.DisableInput` (`self.BP_Player`) _returnvalue)
  (`self.EnableInput` _returnvalue))

(event `EnhancedInput|/Game/Develops/Input/IA/IA_Interact`
  (params (ActionValue :type Boolean) (ElapsedSeconds :type "Float (double-precision)") (TriggeredSeconds :type "Float (double-precision)") (InputAction :type "InputAction Object Reference" :default "/Game/Develops/Input/IA/IA_Interact.IA_Interact"))
  (bind _returnvalue (`GameplayStatics.GetPlayerController` 0))
  (bind _returnvalue_2 (`GameplayStatics.GetPlayerController` 0))
  (:`Triggered`
    (`self.DisableInput` _returnvalue_2)
    (`self.EnableInput` (`self.BP_Player`) _returnvalue_2)
    (bind _wbp_inspection (`self.WBP_Inspection`)
      (:`then`
        (`Widget.RemoveFromParent` _wbp_inspection)
        (set `self.WBP_Inspection` null)
        (`self.K2_DestroyActor`)
        (if (`self.bIsFromUI`)
          (bind _wbp_inventory (`self.WBP_Inventory`)
            (:`then`
              (`WidgetBlueprintLibrary.SetInputMode_UIOnlyEx` _returnvalue _wbp_inventory)
              (set `PlayerController.bShowMouseCursor` true _returnvalue))
            (:`else`))))
      (:`else`))))

(event `EnhancedInput|/Game/Develops/Input/IA/IA_Shoot`
  (params (ActionValue :type Boolean) (ElapsedSeconds :type "Float (double-precision)") (TriggeredSeconds :type "Float (double-precision)") (InputAction :type "InputAction Object Reference" :default "/Game/Develops/Input/IA/IA_Shoot.IA_Shoot"))
  (:`Started`
    (set `self.bCanRotate` true))
  (:`Canceled`
    (set `self.bCanRotate` false :!label _label))
  (:`Completed`
    (goto _label)))

(event `InputAxisKey|MouseX`
  (params (AxisValue :type "Float (single-precision)"))
  (if (`self.bCanRotate`)
    (`SceneComponent.K2_SetWorldRotation` (`self.Item`) (`KismetMathLibrary.ComposeRotators` (`SceneComponent.K2_GetComponentRotation` (`self.Item`)) (`KismetMathLibrary.MakeRotator` 0.0 0.0 (* AxisValue -2.0))) false false)))

(event `InputAxisKey|MouseY`
  (params (AxisValue :type "Float (single-precision)"))
  (if (`self.bCanRotate`)
    (`SceneComponent.K2_SetWorldRotation` (`self.Item`) (`KismetMathLibrary.ComposeRotators` (`SceneComponent.K2_GetComponentRotation` (`self.Item`)) (`KismetMathLibrary.MakeRotator` 0.0 (* AxisValue -2.0))) false false)))

(event `EnhancedInput|/Game/Develops/Input/IA/IA_Move`
  (params (ActionValue :type "Vector2D Structure") (ElapsedSeconds :type "Float (double-precision)") (TriggeredSeconds :type "Float (double-precision)") (InputAction :type "InputAction Object Reference" :default "/Game/Develops/Input/IA/IA_Move.IA_Move"))
  (:`Triggered`
    (`|ExecutionSequence`
      (:`then_0`
        (if (!= ActionValue_X 0.0)
          (`SceneComponent.K2_SetWorldRotation` (`self.Item`) (`KismetMathLibrary.ComposeRotators` (`SceneComponent.K2_GetComponentRotation` (`self.Item`)) (`KismetMathLibrary.MakeRotator` 0.0 0.0 (* ActionValue_X -2.0))) false false)))
      (:`then_1`
        (if (!= ActionValue_Y 0.0)
          (`SceneComponent.K2_SetWorldRotation` (`self.Item`) (`KismetMathLibrary.ComposeRotators` (`SceneComponent.K2_GetComponentRotation` (`self.Item`)) (`KismetMathLibrary.MakeRotator` 0.0 (* ActionValue_Y -2.0))) false false))))))

(event `Key|MouseScrollUp`
  (params (Key :type "Key Structure"))
  (bind _scenecapturecomponent2d (`self.SceneCaptureComponent2D`))
  (:`Pressed`
    (set `SceneCaptureComponent2D.FOVAngle` (`KismetMathLibrary.FClamp` (- (`SceneCaptureComponent2D.FOVAngle` _scenecapturecomponent2d) 3.0) 30.0 100.0) _scenecapturecomponent2d)))

(event `Key|MouseScrollDown`
  (params (Key :type "Key Structure"))
  (bind _scenecapturecomponent2d (`self.SceneCaptureComponent2D`))
  (:`Pressed`
    (set `SceneCaptureComponent2D.FOVAngle` (`KismetMathLibrary.FClamp` (+ (`SceneCaptureComponent2D.FOVAngle` _scenecapturecomponent2d) 3.0) 30.0 100.0) _scenecapturecomponent2d)))

(fn `UserConstructionScript`)