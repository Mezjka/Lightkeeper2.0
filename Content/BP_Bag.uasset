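; BP_Bag is a bag pickup that enlarges the player's inventory.
; Its FuncPickUpBeneficial function casts player character 0 to BP_BaseCharacter, adds two slots to its ACInventory component's slot count and returns true.
; BeginPlay, overlap, Tick and construction only call the parent, so any other behavior is inherited.
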(event `self.ReceiveBeginPlay`
  (`parent.ReceiveBeginPlay`))

(event `self.ReceiveActorBeginOverlap`
  (params (OtherActor :type "Actor Object Reference"))
  (`parent.ReceiveActorBeginOverlap` OtherActor))

(event `self.ReceiveTick`
  (params (DeltaSeconds :type "Float (single-precision)"))
  (`parent.ReceiveTick` DeltaSeconds))

(fn `Func_PickUpBeneficial`
  (returns (Success :type Boolean))
  (bind _asbp_base_character (cast `/Game/BP_BaseCharacter` (`GameplayStatics.GetPlayerCharacter` 0)))
  (bind _ac_inventory (`/Game/BP_BaseCharacter.AC_Inventory` _asbp_base_character))
  (set `/Game/Core/ActorComponents/AC_Inventory.NumberOfSlots` (+ (`/Game/Core/ActorComponents/AC_Inventory.NumberOfSlots` _ac_inventory) 2) _ac_inventory)
  (return true))

(fn `UserConstructionScript`
  (`parent.UserConstructionScript`))